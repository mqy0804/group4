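; Climbable zone actor that lets player character 0 climb while overlapping it.
; On overlap it sets movement to Flying, moves input from the character to itself and adds the Climbing Enhanced Input mapping context.
; Move input drives the character vertically and along its right vector, while jump launches it backward.
; Leaving the overlap sets Falling, restores character input and removes the mapping context.
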(event `self.ReceiveActorBeginOverlap`
  (params (OtherActor :type "Actor Object Reference"))
  (bind _returnvalue (`GameplayStatics.GetPlayerCharacter` 0))
  (bind _returnvalue_2 (`GameplayStatics.GetPlayerController` 0))
  (if (== OtherActor _returnvalue)
    (`CharacterMovementComponent.SetMovementMode` (`Character.CharacterMovement` _returnvalue) "MOVE_Flying" 0)
    (`self.DisableInput` _returnvalue _returnvalue_2)
    (`self.EnableInput` _returnvalue_2)
    (`EnhancedInputSubsystemInterface.AddMappingContext` (pcsubsystem `EnhancedInputLocalPlayerSubsystem` _returnvalue_2) "/Game/AdditionalAssets/WallClimb/Climbing.Climbing" 0 (struct))))

(event `self.ReceiveActorEndOverlap`
  (params (OtherActor :type "Actor Object Reference"))
  (bind _returnvalue (`GameplayStatics.GetPlayerCharacter` 0))
  (bind _returnvalue_2 (`GameplayStatics.GetPlayerController` 0))
  (if (== OtherActor _returnvalue)
    (`CharacterMovementComponent.SetMovementMode` (`Character.CharacterMovement` _returnvalue) "MOVE_Falling" 0)
    (`self.DisableInput` _returnvalue_2)
    (`self.EnableInput` _returnvalue _returnvalue_2)
    (`EnhancedInputSubsystemInterface.RemoveMappingContext` (pcsubsystem `EnhancedInputLocalPlayerSubsystem` _returnvalue_2) "/Game/AdditionalAssets/WallClimb/Climbing.Climbing" (struct))))

(event `EnhancedInput|/Game/Input/Actions/IA_Jump`
  (params (ActionValue :type Boolean) (ElapsedSeconds :type "Float (double-precision)") (TriggeredSeconds :type "Float (double-precision)") (InputAction :type "InputAction Object Reference" :default "/Game/Input/Actions/IA_Jump.IA_Jump"))
  (bind _returnvalue (`GameplayStatics.GetPlayerCharacter` 0))
  (:`Started`
    (`Character.LaunchCharacter` _returnvalue (* (`self.GetActorForwardVector` _returnvalue) -1 1500.0) true false)))

(event `EnhancedInput|/Game/Input/Actions/IA_Move`
  (params (ActionValue :type "Vector2D Structure") (ElapsedSeconds :type "Float (double-precision)") (TriggeredSeconds :type "Float (double-precision)") (InputAction :type "InputAction Object Reference" :default "/Game/Input/Actions/IA_Move.IA_Move"))
  (bind _returnvalue (`GameplayStatics.GetPlayerCharacter` 0))
  (:`Triggered`
    (`Pawn.AddMovementInput` _returnvalue (0.0 0.0 1.0) ActionValue_Y false)
    (`Pawn.AddMovementInput` _returnvalue (`self.GetActorRightVector` _returnvalue) ActionValue_X false)))

(fn `UserConstructionScript`)